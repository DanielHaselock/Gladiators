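; BP_EnnemyBar is an enemy actor Blueprint that shows life through a WBP_EnnemyBar hosted in its Widget component.
; On BeginPlay it copies MaxLife into the widget and starts the widget's Life at that maximum.
; Every Tick it casts the widget again and pushes the actor's current Life into it, polling rather than reacting to change events.
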(event `self.ReceiveBeginPlay`
  (bind _aswbp_ennemy_bar (cast `/Game/WBP_EnnemyBar` (`WidgetComponent.GetWidget` (`self.Widget`))))
  (bind _output_get (set `/Game/WBP_EnnemyBar.MaxLife` (`self.MaxLife`) _aswbp_ennemy_bar))
  (set `/Game/WBP_EnnemyBar.Life` _output_get _aswbp_ennemy_bar))

(event `self.ReceiveTick`
  (params (DeltaSeconds :type "Float (single-precision)"))
  (bind _aswbp_ennemy_bar (cast `/Game/WBP_EnnemyBar` (`WidgetComponent.GetWidget` (`self.Widget`))))
  (set `/Game/WBP_EnnemyBar.Life` (`self.Life`) _aswbp_ennemy_bar))

(fn `UserConstructionScript`)