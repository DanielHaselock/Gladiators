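; BP_Enemy is an enemy character with a hammer hit collision and a life bar, both held as child actors.
; BeginPlay flags the hammer collision as enemy-owned, and Tick copies the enemy's attacking state to it.
; The construction script fills the bar from the Damage component's MaxLife.
; Tick then updates its Life and yaws it toward the first player's camera, billboard-style.
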(event `self.ReceiveBeginPlay`
  (bind _asbp_hammer_hit_collision (cast `/Game/BP_HammerHitCollision` (`ChildActorComponent.ChildActor` (`self.BP_HammerHitCollision`))))
  (bind _output_get (set `self.HammerCollision` _asbp_hammer_hit_collision))
  (set `HammerHitCollision.IsEnemy` true _output_get))

(event `self.ReceiveTick`
  (params (DeltaSeconds :type "Float (single-precision)"))
  (bind _childactor (`ChildActorComponent.ChildActor` (`self.BP_EnnemyBar`)))
  (bind (_returnvalue_roll _returnvalue_pitch _returnvalue_yaw) (`KismetMathLibrary.BreakRotator` (`KismetMathLibrary.FindLookAtRotation` (`self.K2_GetActorLocation` _childactor) (`PlayerCameraManager.GetCameraLocation` (`PlayerController.PlayerCameraManager` (`GameplayStatics.GetPlayerController` 0))))))
  (bind _output_get (set `self.IsAttacking` (`self.IsAttackingEnemy`)))
  (set `HammerHitCollision.IsAttacking` _output_get (`self.HammerCollision`))
  (`self.K2_SetActorRotation` _childactor (`KismetMathLibrary.MakeRotator` 0.0 0.0 _returnvalue_yaw) false)
  (bind _asbp_ennemy_bar (cast `/Game/BP_EnnemyBar` (`ChildActorComponent.ChildActor` (`self.BP_EnnemyBar`))))
  (set `/Game/BP_EnnemyBar.Life` (`DamageComponent.Life` (`self.Damage`)) _asbp_ennemy_bar))

(fn `UserConstructionScript`
  (bind _asbp_ennemy_bar (cast `/Game/BP_EnnemyBar` (`ChildActorComponent.ChildActor` (`self.BP_EnnemyBar`))))
  (bind _output_get (set `/Game/BP_EnnemyBar.MaxLife` (`DamageComponent.MaxLife` (`self.Damage`)) _asbp_ennemy_bar))
  (set `/Game/BP_EnnemyBar.Life` _output_get _asbp_ennemy_bar))